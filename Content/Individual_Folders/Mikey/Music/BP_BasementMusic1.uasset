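; Trigger actor that plays basement music, with loudness driven by how deep the player descends.
; The first time the player character overlaps its Box, it spawns a 2D point-of-interest sound through a DoOnce.
; Tick then continually adjusts that sound's volume from the player pawn's Z, rising as height drops.
; The height mapping is unclamped, so volume extrapolates beyond the set range.
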(event `self.ReceiveTick`
  (params (DeltaSeconds :type "Float (single-precision)"))
  (`/Engine/EditorBlueprintResources/StandardMacros.IsValid` (stale `self.Box.OnComponentBeginOverlap` _returnvalue) :!label _label
    (:`Is Valid`
      (`AudioComponent.AdjustVolume` (stale `self.Box.OnComponentBeginOverlap` _returnvalue) 0.1 (`KismetMathLibrary.MapRangeUnclamped` (.z (`self.K2_GetActorLocation` (`GameplayStatics.GetPlayerPawn` 0))) -201.0 -1300.0 0.0 2.0) "Linear"))))

(event `self.Box.OnComponentBeginOverlap`
  (params (OverlappedComponent :type "PrimitiveComponent Object Reference") (OtherActor :type "Actor Object Reference") (OtherComp :type "PrimitiveComponent Object Reference") (OtherBodyIndex :type Integer) (bFromSweep :type Boolean) (SweepResult :type "HitResult Structure (by ref)"))
  (if (== OtherActor (`GameplayStatics.GetPlayerCharacter` 0))
    (`/Engine/EditorBlueprintResources/StandardMacros.DoOnce` false
      (:`Completed`
        (bind _returnvalue (`GameplayStatics.SpawnSound2D` "/Game/Individual_Folders/Mikey/Music/SoundWaves/1S_PointOfInterest2.1S_PointOfInterest2" (`KismetMathLibrary.MapRangeUnclamped` (.z (`self.K2_GetActorLocation` (`GameplayStatics.GetPlayerPawn` 0))) -201.0 -1300.0 0.0 2.0) 1.0 0.0 null))
        (goto _label)))))

(fn `UserConstructionScript`)