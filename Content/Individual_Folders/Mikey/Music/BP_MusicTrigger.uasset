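; BP_MusicTrigger is a box trigger that sets which music track plays when the player character walks into it.
; It finds BP_MusicManager in the level on BeginPlay and checks its state on each player overlap.
; If no music is playing, it plays SelectedMusicTrack through the manager.
; If a different track is playing, it calls the manager's change-track dispatcher with both tracks, and an already matching track is left alone.
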(event `self.ReceiveBeginPlay`
  (bind _returnvalue (`GameplayStatics.GetActorOfClass` "/Game/Individual_Folders/Mikey/Music/BP_MusicManager.BP_MusicManager_C")))

(event `self.BoxCollision.OnComponentBeginOverlap`
  (params (OverlappedComponent :type "PrimitiveComponent Object Reference") (OtherActor :type "Actor Object Reference") (OtherComp :type "PrimitiveComponent Object Reference") (OtherBodyIndex :type Integer) (bFromSweep :type Boolean) (SweepResult :type "HitResult Structure (by ref)"))
  ;[1 1 1] Collision w Player
  (if (== OtherActor (`GameplayStatics.GetPlayerCharacter` 0))
    (if (`/Game/Individual_Folders/Mikey/Music/BP_MusicManager.isMusicPlaying` (stale `self.ReceiveBeginPlay` _returnvalue))
      (if (not (== (`/Game/Individual_Folders/Mikey/Music/BP_MusicManager.CurrentlyPlayingTrack` (stale `self.ReceiveBeginPlay` _returnvalue)) (`self.SelectedMusicTrack`)))
        (`/Game/Individual_Folders/Mikey/Music/BP_MusicManager.ChangeMusicTrackDispatcher` (stale `self.ReceiveBeginPlay` _returnvalue) (`/Game/Individual_Folders/Mikey/Music/BP_MusicManager.CurrentlyPlayingTrack` (stale `self.ReceiveBeginPlay` _returnvalue)) (`self.SelectedMusicTrack`)))
      (else
        (`/Game/Individual_Folders/Mikey/Music/BP_MusicManager.PlayTrack` (stale `self.ReceiveBeginPlay` _returnvalue) (`self.SelectedMusicTrack`)) ; Calls the play track function in the music manager
      ))))

(fn `UserConstructionScript`)